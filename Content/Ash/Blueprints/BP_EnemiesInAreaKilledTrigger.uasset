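; Trigger Blueprint that signals when every enemy in its EnemiesInArea array has been killed.
; Each Tick it loops over the array, calling Remove on the BP_FishGoblin cast result when health is at or below zero, the entry is invalid, or the cast fails.
; It fires EnemiesInAreaKilled on every Tick that the array is empty, with no one-shot guard.
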(event EventTick
  (params (DeltaSeconds :type Float%20%28single-precision%29))
  (for _array_element (Variables|Default|GetEnemiesInArea)
    (Utilities|IsValid _array_element
      (:Is%20Valid
        (bind _asbp_fish_goblin (Utilities|Casting|CastToBP_FishGoblin _array_element)
          (:then
            (if (<= (Variables|/Game/Ash/Blueprints/Components/HealthComponent.HealthComponent_C|GetCurrentHealth (Variables|/Game/Ash/Blueprints/Enemies/BP_FishGoblin.BP_FishGoblin_C|GetHealthComponent _asbp_fish_goblin)) 0.0)
              (Utilities|Array|RemoveItem (Variables|Default|GetEnemiesInArea) _asbp_fish_goblin :!label _label)))
          (:CastFailed
            (goto _label))))
      (:Is%20Not%20Valid
        (goto _label))))
  (if (<= (Utilities|Array|Length (Variables|Default|GetEnemiesInArea)) 0)
    (Default|CallEnemiesinAreaKilled)))

(fn ConstructionScript)