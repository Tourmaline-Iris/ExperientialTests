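; Test NPC that plays a short, hardcoded two-line placeholder dialogue when Talk fires.
; Talk creates the dialogue HUD, fills ConversationText and writes the first line, keeping the returned index for the next.
; The HUD's FinishedWriting delegate chains the steps: ContinueDialogue writes the next line, then binds EndDialogue to exit.
; Each step adds its binding without removing the previous one in this graph.
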(event Custom|EndDialogue
  (CallFunction|ExitDialogue (stale EventTalk _dialoguehud)))

(event Custom|ContinueDialogue
  (CallFunction|WriteDialogueText (Variables|Default|GetConversation%20Text) (stale EventTalk _dialoguehud) (stale EventTalk _nextindex))
  (EventDispatchers|AssignFinishedWriting (stale EventTalk _dialoguehud) (delegate Custom|EndDialogue)))

(event EventTalk
  (bind _conversation_text (Variables|Default|GetConversation%20Text))
  (bind _dialoguehud (CallFunction|DrawDialogueHUD))
  (CallFunction|AddDialogueTexttoArray _conversation_text "This is a test. I should probably be saying something 
interesting but I've been told I won't make it into the final 
game so why bother.")
  (CallFunction|AddDialogueTexttoArray _conversation_text "My life is meaningless...")
  (bind _nextindex (CallFunction|WriteDialogueText _conversation_text _dialoguehud))
  (EventDispatchers|AssignFinishedWriting _dialoguehud (delegate Custom|ContinueDialogue)))

(fn ConstructionScript)