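; BP_Mango is the Pirate Island quest NPC Mango, progressing from rescue through a kitchen fruit task to Mirabelle's quest.
; Bound trigger events and stage events swap BPCompDialogue's trees and trigger actors, while toggling the mesh's GameTraceChannel3 response gates when it can be traced.
; Once Mirabelle is helped, it teleports both characters to dialogue triggers and spawns an auto-interact actor, then switches to post-quest dialogue on completion.
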(event Custom|PlayerSavesMango
  (bind _dialoguetrigger1 (Variables|Default|GetDialogueTrigger1))
  (Variables|Default|SetTerrified false)
  (Collision|SetCollisionResponsetoChannel (Variables|Character|GetMesh) "ECC_GameTraceChannel3" "ECR_Block")
  (Variables|/Game/Billy/DialogueSystemMKII/BPComp_Dialogue.BPComp_Dialogue_C|SetActorToTrigger1 (Variables|Default|GetBPComp_Dialogue) _dialoguetrigger1)
  (EventDispatchers|BindEventtoPlayerMetMango _dialoguetrigger1 (delegate Custom|RunningToKitchen)))

(event Custom|MangoNeedsHelp
  (Variables|Default|SetTerrified true)
  (Collision|SetCollisionResponsetoChannel (Variables|Character|GetMesh) "ECC_GameTraceChannel3" "ECR_Ignore")
  (EventDispatchers|BindEventtoEnemiesinAreaKilled (Variables|Default|GetEnemiesKilledTrigger) (delegate Custom|PlayerSavesMango)))

(event Custom|RunningToKitchen
  (Collision|SetCollisionResponsetoChannel (Variables|Character|GetMesh) "ECC_GameTraceChannel3" "ECR_Ignore"))

(event Custom|ReachedKitchen
  (params (FruitBasket :type BP%20Fruit%20Basket%20Object%20Reference))
  (EventDispatchers|BindEventtoPlayerPutFruitinBasket FruitBasket (delegate Custom|AllFruitInBasket))
  (if (Variables|/Game/Ash/Blueprints/LevelSpecific/PirateIsland/BP_FruitBasket.BP_FruitBasket_C|GetPlayerFruitPresent FruitBasket)
    (CallFunction|AllFruitinBasket)
    (else
      (Variables|/Game/Billy/DialogueSystemMKII/BPComp_Dialogue.BPComp_Dialogue_C|SetDialogueTree (Variables|Default|GetBPComp_Dialogue) "/Game/Ash/Blueprints/LevelSpecific/PirateIsland/BT_MangoRunningToKitchen.BT_MangoRunningToKitchen")
      (Collision|SetCollisionResponsetoChannel (Variables|Character|GetMesh) "ECC_GameTraceChannel3" "ECR_Block"))))

(event Custom|AllFruitInBasket
  (bind _bpcomp_dialogue (Variables|Default|GetBPComp_Dialogue))
  (Utilities|FlowControl|DoOnce false
    (:Completed
      (Variables|/Game/Billy/DialogueSystemMKII/BPComp_Dialogue.BPComp_Dialogue_C|SetDialogueTree _bpcomp_dialogue "/Game/Ash/Blueprints/LevelSpecific/PirateIsland/BT_MangoAsksForHelp.BT_MangoAsksForHelp")
      (Variables|/Game/Billy/DialogueSystemMKII/BPComp_Dialogue.BPComp_Dialogue_C|SetActorToTrigger3 _bpcomp_dialogue (Variables|Default|GetDialogueTrigger3))
      (Variables|/Game/Billy/DialogueSystemMKII/BPComp_Dialogue.BPComp_Dialogue_C|SetActorToTrigger2 _bpcomp_dialogue (Variables|Default|GetDialogueTrigger2))
      (Collision|SetCollisionResponsetoChannel (Variables|Character|GetMesh) "ECC_GameTraceChannel3" "ECR_Block"))))

(event Custom|PlayerHelpedMirabelle
  (bind _bpcomp_dialogue (Variables|Default|GetBPComp_Dialogue))
  (bind _dialoguetrigger4 (Variables|Default|GetDialogueTrigger4))
  (bind _dialoguetrigger5 (Variables|Default|GetDialogueTrigger5))
  (bind _returnvalue (Transformation|GetActorLocation _dialoguetrigger4))
  (bind _returnvalue_2 (Transformation|GetActorLocation _dialoguetrigger5))
  (Variables|/Game/Billy/DialogueSystemMKII/BPComp_Dialogue.BPComp_Dialogue_C|SetDialogueTree _bpcomp_dialogue "/Game/Ash/Blueprints/LevelSpecific/PirateIsland/BT_ReturningToReality.BT_ReturningToReality")
  (Variables|/Game/Billy/DialogueSystemMKII/BPComp_Dialogue.BPComp_Dialogue_C|SetActorToTrigger4 _bpcomp_dialogue (Variables|Default|GetDialogueTrigger4))
  (Variables|/Game/Billy/DialogueSystemMKII/BPComp_Dialogue.BPComp_Dialogue_C|SetActorToTrigger5 _bpcomp_dialogue (Variables|Default|GetDialogueTrigger5))
  (Transformation|SetActorLocationAndRotation (Math|Vector|MakeVector (.x _returnvalue) (.y _returnvalue) 1.48e+03) (Transformation|GetActorRotation _dialoguetrigger4) false true)
  (Transformation|SetActorLocationAndRotation (Variables|Default|GetMirabelleRef) (Math|Vector|MakeVector (.x _returnvalue_2) (.y _returnvalue_2) 1476.0) (Transformation|GetActorRotation _dialoguetrigger5) false true)
  (Utilities|FlowControl|Delay 0.2)
  (bind _asfirst_person_character (Utilities|Casting|CastToFirstPersonCharacter (Game|GetPlayerCharacter 0)))
  (Game|SpawnActorfromClass "/Game/Ash/Blueprints/LevelSpecific/PirateIsland/BP_TriggerInteractOnSpawn.BP_TriggerInteractOnSpawn_C" (Transformation|GetActorTransform) "AlwaysSpawn" 0 self _asfirst_person_character 0)
  (EventDispatchers|BindEventtoMirabelle'sSunconsciousQuestComplete (Variables|Default|GetDialogueTrigger5) (delegate Custom|QuestComplete)))

(event Custom|QuestComplete
  (Variables|/Game/Billy/DialogueSystemMKII/BPComp_Dialogue.BPComp_Dialogue_C|SetDialogueTree (Variables|Default|GetBPComp_Dialogue) "/Game/Ash/Blueprints/LevelSpecific/PirateIsland/BT_MangoPostQuest.BT_MangoPostQuest"))

(fn ConstructionScript
  (|CallParentFunction))