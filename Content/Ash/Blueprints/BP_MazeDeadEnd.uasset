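; Maze dead-end actor: a standing male figure with looping whispers that fades away and destroys itself when the player enters its box.
; A self-repeating delayed event slides the whisper audio to the spline point nearest the player.
; A per-tick line trace from the audio to the player lowers its volume when blocked.
; On overlap, a timeline drives dither on dynamic materials and the whisper volume multiplier.
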(event OnComponentBeginOverlap(Box)
  (params (OverlappedComponent :type Primitive%20Component%20Object%20Reference) (OtherActor :type Actor%20Object%20Reference) (OtherComp :type Primitive%20Component%20Object%20Reference) (OtherBodyIndex :type Integer) (bFromSweep :type Boolean) (SweepResult :type Hit%20Result%20Structure%20%28by%20ref%29))
  ;[1 1 1] Fade away
  (if (== OtherActor (Game|GetPlayerCharacter 0))
    (bind _ditheramount (Timeline|DitherMesh Play)
      (:Update
        (for _array_element (Variables|Default|GetDynamicMaterials)
          (Rendering|Material|SetScalarParameterValue _array_element "DitherPercent" _ditheramount :!class /Script/Engine.MaterialInstanceDynamic)
          (Audio|Components|Audio|SetVolumeMultiplier (Variables|Default|Getwhispers-loop_Cue) _ditheramount :!class /Script/Engine.AudioComponent)))
      (:Finished
        (Actor|DestroyActor)))))

(event Custom|MoveAudio
  ;[1 1 1] Move audio cue along spline
  (Transformation|SetWorldLocation (Variables|Default|Getwhispers-loop_Cue) (Spline|FindLocationClosesttoWorldLocation (Variables|Default|GetSpline) (Transformation|GetActorLocation (Variables|Default|GetPlayerReference)) "World") false false)
  (Utilities|FlowControl|Delay 0.05)
  (CallFunction|MoveAudio))

(event EventBeginPlay
  (bind _asfirst_person_character (Utilities|Casting|CastToFirstPersonCharacter (Game|GetPlayerCharacter 0)))
  (Variables|Default|SetPlayerReference _asfirst_person_character)
  (CallFunction|MoveAudio)
  ;[1 1 1] Create dynamic material instances
  (for _array_element (Rendering|Material|GetMaterials (Variables|Default|GetMale_Standing_Pose))
    (bind _returnvalue (Rendering|Material|CreateDynamicMaterialInstance _array_element "None" "None" :!class /Script/Engine.KismetMaterialLibrary))
    (bind _returnvalue_2 (Utilities|Array|Add (Variables|Default|GetDynamicMaterials) _returnvalue))
    (Rendering|Material|SetMaterial (Variables|Default|GetMale_Standing_Pose) _returnvalue_2 _returnvalue)))

(event EventTick
  (params (DeltaSeconds :type Float%20%28single-precision%29))
  (bind _whispers_loop_cue (Variables|Default|Getwhispers-loop_Cue))
  ;[1 1 1] Don't play through walls
  (bind _outhit (Collision|LineTraceForObjects (Transformation|GetWorldLocation (Variables|Default|Getwhispers-loop_Cue)) (Transformation|GetActorLocation (Variables|Default|GetPlayerReference)) (Utilities|Array|MakeArray "ObjectTypeQuery3" "ObjectTypeQuery1") false 0 "None" true "(R=1.000000,G=0.000000,B=0.000000,A=1.000000)" "(R=0.000000,G=1.000000,B=0.000000,A=1.000000)" DeltaSeconds))
  (if (and (Utilities|IsValid (.HitActor (Collision|BreakHitResult _outhit))) (== (.HitActor (Collision|BreakHitResult _outhit)) (Variables|Default|GetPlayerReference)))
    (Audio|Components|Audio|AdjustVolume _whispers_loop_cue 0.5 1.0 "Linear" :!class /Script/Engine.AudioComponent)
    (else
      (Audio|Components|Audio|AdjustVolume _whispers_loop_cue 0.5 0.001 "Linear" :!class /Script/Engine.AudioComponent))))

(fn ConstructionScript)