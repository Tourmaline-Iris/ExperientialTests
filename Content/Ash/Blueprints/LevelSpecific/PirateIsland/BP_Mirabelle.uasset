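; Mirabelle NPC for the Pirate Island level, who moves between a bedroom and a mango room.
; On BeginPlay, after a successful game instance cast, she teleports to a spot offset from the bedroom move point.
; Two custom events drive AI MoveTo toward each room's point, calling themselves again on failure.
; The bedroom run disables the door's collision and restores it only once the move succeeds.
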(event Custom|RunToBedroom
  (Collision|SetActorEnableCollision (Variables|Default|GetBedroomDoor) false)
  (AI|AIMoveTo self "0, 0, 0" (Variables|Default|GetBedroomMoveToPoint) 5.0 true
    (:OnSuccess
      (Collision|SetActorEnableCollision (Variables|Default|GetBedroomDoor) true))
    (:OnFail
      (CallFunction|RuntoBedroom))))

(event Custom|RunToMangoRoom
  (AI|AIMoveTo self "0, 0, 0" (Variables|Default|GetMangoRoomMoveToPoint) 5.0 true
    (:OnFail
      (CallFunction|RuntoMangoRoom))))

(event EventBeginPlay
  (bind _bedroommovetopoint (Variables|Default|GetBedroomMoveToPoint))
  (bind _returnvalue (Transformation|GetActorLocation _bedroommovetopoint))
  (bind _asgi_hero_adrift (Utilities|Casting|CastToGI_HeroAdrift (Game|GetGameInstance)))
  (Transformation|SetActorLocation (Math|Vector|MakeVector (.x _returnvalue) (- (.y _returnvalue) 1.5e+02) (.z _returnvalue)) false true))

(fn ConstructionScript)