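; BP_Door is a physics-driven door that swings itself back to its closed rotation after being hit.
; The construction script records the closed rotation, and each component hit retriggers a three-second delay before physics is switched off.
; A timeline then interpolates from the current rotation to closed along the shortest path, re-enabling physics shortly after it finishes.
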(event OnComponentHit(Door)
  (params (HitComponent :type Primitive%20Component%20Object%20Reference) (OtherActor :type Actor%20Object%20Reference) (OtherComp :type Primitive%20Component%20Object%20Reference) (NormalImpulse :type Vector :default "0, 0, 0") (Hit :type Hit%20Result%20Structure%20%28by%20ref%29))
  (bind _door (Variables|Default|GetDoor))
  (Utilities|FlowControl|RetriggerableDelay 3.0)
  (Physics|SetSimulatePhysics _door false)
  (Variables|Default|SetOpenRot (Transformation|GetWorldRotation _door))
  (bind _newtrack_0 (Timeline|Timeline_0 PlayFromStart)
    (:Update
      (Transformation|SetWorldRotation (Variables|Default|GetDoor) (Math|Rotator|Lerp(Rotator) (Variables|Default|GetOpenRot) (Variables|Default|GetClosedRot) _newtrack_0 true) false false))
    (:Finished
      (Utilities|FlowControl|Delay 0.1)
      (Physics|SetSimulatePhysics (Variables|Default|GetDoor) true))))

(fn ConstructionScript
  (Variables|Default|SetClosedRot (Transformation|GetWorldRotation (Variables|Default|GetDoor))))