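; Base NPC Blueprint for conversations, providing shared dialogue helpers and turning the NPC to face the player when talked to.
; Talk stores the player reference and runs a timeline that lerps only the actor's yaw toward player character 0.
; Helper functions create the DialogueHUD, append lines, and start timed typing of the indexed line unless one is already writing.
; ExitDialogue hands the widget back to the FirstPersonCharacter to end the conversation.
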(event Custom|Talk
  (params (Player :type Object%20Object%20Reference))
  (Variables|Default|SetPlayerRef Player)
  ;[1 1 1] Face Player
  (bind _look_at_player_track (Timeline|Look%20At%20Player PlayFromStart)
    (:Update
      (Transformation|SetActorRotation (Math|Rotator|MakeRotator 0.0 0.0 (.yaw (Math|Rotator|Lerp(Rotator) (Transformation|GetActorRotation) (Math|Rotator|FindLookatRotation (Transformation|GetActorLocation) (Transformation|GetActorLocation (Game|GetPlayerCharacter 0))) _look_at_player_track true)))))))

(fn ConstructionScript)

(fn DrawDialogueHUD
  (bind _returnvalue (UserInterface|CreateWidget "/Game/Ash/Blueprints/Widgets/DialogueHUD.DialogueHUD_C" (Game|GetPlayerController 0) (Variables|Default|GetNPC_CharsPerSecond)))
  (UserInterface|Viewport|AddtoViewport _returnvalue 0)
  (bind _output_get (Variables|Default|SetDialogueHUD _returnvalue))
  (return _output_get))

(fn WriteDialogueText
  (params (ConversationText :type Array%20of%20Strings) (DialogueHUD :type Dialogue%20HUD%20Object%20Reference) (IndexToDisplay :type Integer))
  (LocalVariables|SetTextToWrite (Utilities|Array|Get(acopy) ConversationText IndexToDisplay))
  (bind _asdialogue_hud (Utilities|Casting|CastToDialogueHUD DialogueHUD))
  ;[1 1 1] Clear dialogue box
  (Rendering|Components|TextRender|SetText (Variables|/Game/Ash/Blueprints/Widgets/DialogueHUD.DialogueHUD_C|GetRichTextBlock_Dialogue _asdialogue_hud) (LocalVariables|GetBlankText))
  ;[1 1 1] Tell DialogueHUD to type text
  (Variables|/Game/Ash/Blueprints/Widgets/DialogueHUD.DialogueHUD_C|SetCharsPerSecond _asdialogue_hud (Variables|Default|GetNPC_CharsPerSecond))
  (if (not (Variables|/Game/Ash/Blueprints/Widgets/DialogueHUD.DialogueHUD_C|GetIsWriting _asdialogue_hud))
    (Variables|/Game/Ash/Blueprints/Widgets/DialogueHUD.DialogueHUD_C|SetText _asdialogue_hud (LocalVariables|GetTextToWrite))
    (Variables|/Game/Ash/Blueprints/Widgets/DialogueHUD.DialogueHUD_C|SetIsWriting _asdialogue_hud true)
    (Variables|/Game/Ash/Blueprints/Widgets/DialogueHUD.DialogueHUD_C|SetStartTimestamp _asdialogue_hud (Utilities|Time|GetGameTimeinSeconds))
    (return (+ IndexToDisplay 1))))

(fn AddDialogueTexttoArray
  (params (TargetArray :type Array%20of%20Strings) (TextToAdd :type String))
  (Utilities|Array|Add TargetArray TextToAdd)
  (return TargetArray))

(fn ExitDialogue
  (params (DialogueWidget :type Dialogue%20HUD%20Object%20Reference))
  (bind _asfirst_person_character (Utilities|Casting|CastToFirstPersonCharacter (Variables|Default|GetPlayerRef)))
  (Default|EndDialogue _asfirst_person_character DialogueWidget))