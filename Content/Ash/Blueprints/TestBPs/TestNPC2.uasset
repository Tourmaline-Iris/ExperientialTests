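; Test NPC that plays a fixed, three-line placeholder conversation when the player talks to it.
; Talk calls the parent, draws the dialogue HUD, fills the ConversationText array and writes the first line.
; Chained custom events bound to the HUD's finished-writing event show each next line using the index returned by the previous write, then exit the dialogue.
; Only the first continue handler is unbound; later bindings are left in place.
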(event Custom|EndDialogue
  (CallFunction|ExitDialogue (Variables|Default|GetDialogueHUD)))

(event Custom|ContinueDialogue2
  (bind _dialoguehud (Variables|Default|GetDialogueHUD))
  (CallFunction|WriteDialogueText (Variables|Default|GetConversationText) _dialoguehud (stale Custom|ContinueDialogue _nextindex))
  (EventDispatchers|BindEventtoFinishedWriting _dialoguehud (delegate Custom|EndDialogue)))

(event Custom|ContinueDialogue
  (bind _dialoguehud (Variables|Default|GetDialogueHUD))
  (bind _nextindex (CallFunction|WriteDialogueText (Variables|Default|GetConversationText) _dialoguehud (stale EventTalk _nextindex)))
  (EventDispatchers|UnbindEventfromFinishedWriting _dialoguehud (delegate Custom|ContinueDialogue))
  (EventDispatchers|BindEventtoFinishedWriting _dialoguehud (delegate Custom|ContinueDialogue2)))

(event EventTalk
  (params (Player :type Object%20Object%20Reference))
  (bind _conversationtext (Variables|Default|GetConversationText))
  (|CallParentFunction Player)
  (bind _dialoguehud (CallFunction|DrawDialogueHUD))
  (CallFunction|AddDialogueTexttoArray _conversationtext "Woo I've been migrated!")
  (CallFunction|AddDialogueTexttoArray _conversationtext "This is a test. I should probably be saying something 
interesting but I've been told I won't make it into the final 
game so why bother.")
  (bind _textarray (CallFunction|AddDialogueTexttoArray _conversationtext "My life is meaningless..."))
  (bind _nextindex (CallFunction|WriteDialogueText _textarray _dialoguehud))
  (EventDispatchers|BindEventtoFinishedWriting _dialoguehud (delegate Custom|ContinueDialogue)))

(fn ConstructionScript
  (|CallParentFunction))