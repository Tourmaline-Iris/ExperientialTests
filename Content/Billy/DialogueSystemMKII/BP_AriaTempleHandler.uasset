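; BP_AriaTempleHandler sets up the Aria temple's layout on BeginPlay from the player's saved state in GI_HeroAdrift.
; LoadPlants shows talkable plants and blocks their trace channel only if the player has the talk-to-plants ability, otherwise hiding and ignoring them.
; The first unfinished DruidIslandProgress step selects a hidden-state array.
; SetObjectsVisibility applies it by index to visibility and collision of actors attached to each ObjectsToChange entry.
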(event EventLoadPlants
  (bind _plantscontainer (Variables|Default|GetPlantsContainer))
  (bind _outactors (Actor|GetAttachedActors _plantscontainer true))
  (if (Variables|/Game/Ash/Blueprints/GI_HeroAdrift.GI_HeroAdrift_C|GetPlayerHasTalkToPlants (.AsGI%20Hero%20Adrift (Utilities|Casting|CastToGI_HeroAdrift (Game|GetGameInstance))))
    (for _array_element _outactors
      (Rendering|SetActorHiddenInGame _array_element false)
      (bind _asbp_plant_talkable (Utilities|Casting|CastToBP_PlantTalkable _array_element))
      (Collision|SetCollisionResponsetoChannel (Variables|/Game/Billy/DialogueSystemMKII/BP_PlantTalkable.BP_PlantTalkable_C|GetSphere _asbp_plant_talkable) "ECC_GameTraceChannel3" "ECR_Block"))
    (else
      (for _array_element_2 _outactors
        (Rendering|SetActorHiddenInGame _array_element_2 true)
        (bind _asbp_plant_talkable_2 (Utilities|Casting|CastToBP_PlantTalkable _array_element_2))
        (Collision|SetCollisionResponsetoChannel (Variables|/Game/Billy/DialogueSystemMKII/BP_PlantTalkable.BP_PlantTalkable_C|GetSphere _asbp_plant_talkable_2) "ECC_GameTraceChannel3" "ECR_Ignore")))))

(event EventUpdateLevelProgress
  (bind _array (Utilities|Array|MakeArray true true))
  (bind _array_2 (Utilities|Array|MakeArray false false))
  (bind (_progressindex _arrayhasfalse) (CallFunction|GetProgress))
  (if _arrayhasfalse
    (bind _result (Math|Integer|DecrementInt _progressindex)
      (:%20%20
        (switch int _result
          (:Default
            (Variables|Default|SetObjectStateArray (Utilities|Array|MakeArray false false false)))
          (:0
            (CallFunction|LoadPlants)
            (Variables|Default|SetObjectStateArray _array_2))
          (:1
            (Variables|Default|SetObjectStateArray _array_2))
          (:2
            (Variables|Default|SetObjectStateArray (Utilities|Array|MakeArray false false)))
          (:3
            (Variables|Default|SetObjectStateArray (Utilities|Array|MakeArray true false)))
          (:4
            (Variables|Default|SetObjectStateArray _array))
          (:5
            (Variables|Default|SetObjectStateArray _array :!label _label)))))
    (else
      (goto _label)))
  (bind _values (Utilities|Map|Values (Variables|Default|GetObjectsToChange)))
  (CallFunction|SetObjectsVisibility (Variables|Default|GetObjectStateArray) _values))

(event EventChangeLayoutonEntry
  (bind _values (Utilities|Map|Values (Variables|Default|GetObjectsToChange)))
  (CallFunction|SetObjectsVisibility (Variables|Default|GetObjectStateArray) _values))

(event EventBeginPlay
  (CallFunction|LoadPlants)
  (CallFunction|UpdateLevelProgress)
  (CallFunction|ChangeLayoutonEntry))

(fn ConstructionScript)

(fn SetObjectsVisibility
  (params (IsHidden :type Array%20of%20Booleans) (Objects :type Array%20of%20Actor%20Object%20References))
  (for (_array_element _array_index) Objects
    (for _array_element_2 (Actor|GetAttachedActors _array_element true)
      (Rendering|SetActorHiddenInGame _array_element_2 (Utilities|Array|Get(acopy) IsHidden _array_index))
      (Collision|SetActorEnableCollision _array_element_2 (not (Utilities|Array|Get(acopy) IsHidden _array_index))))))

(fn GetProgress
  (bind _values (Utilities|Map|Values (Variables|/Game/Ash/Blueprints/GI_HeroAdrift.GI_HeroAdrift_C|GetDruidIslandProgress (.AsGI%20Hero%20Adrift (Utilities|Casting|CastToGI_HeroAdrift (Game|GetGameInstance))))))
  (return (Utilities|Array|FindItem _values false) (Utilities|Array|ContainsItem _values false)))