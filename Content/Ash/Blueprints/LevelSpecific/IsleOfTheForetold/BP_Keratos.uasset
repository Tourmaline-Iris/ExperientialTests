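; Keratos, a dialogue NPC on the Isle of the Foretold who starts seated.
; On BeginPlay he hands five trigger actors to his dialogue component and picks the full or short monologue tree from the RangarLeft progress flag in the game instance.
; Stand uses a timeline to move him toward the first trigger object's X and Z, ignoring WorldDynamic collision until finished.
; UnsheatheSword snaps his sword to a finger socket.
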(event Custom|UnsheatheSword
  (Transformation|AttachComponentToComponent (Variables|Default|GetSword) (Variables|Character|GetMesh) "FingerMiddle_01_RSocket" "SnapToTarget" "SnapToTarget" "SnapToTarget" true))

(event Custom|Stand
  (bind _returnvalue (Transformation|GetActorLocation))
  (bind _returnvalue_2 (Transformation|GetActorLocation))
  (Collision|SetCollisionResponsetoChannel (Variables|Default|GetCapsuleComponent) "ECC_WorldDynamic" "ECR_Ignore")
  (bind (_direction _lerp_z _lerp_forward) (Timeline|Timeline_0 PlayFromStart)
    (:Update
      (Transformation|SetActorLocation (Math|Vector|Lerp(Vector) (Math|Vector|MakeVector (.x _returnvalue) (.y _returnvalue) (.z _returnvalue)) (Math|Vector|MakeVector (.x _returnvalue) (.y _returnvalue) (.z (Transformation|GetActorLocation (Variables|Default|GetDialogueTriggerObject1)))) _lerp_z) false false)
      (Transformation|SetActorLocation (Math|Vector|Lerp(Vector) (Math|Vector|MakeVector (.x _returnvalue_2) (.y _returnvalue_2) (.z _returnvalue_2)) (Math|Vector|MakeVector (.x (Transformation|GetActorLocation (Variables|Default|GetDialogueTriggerObject1))) (.y _returnvalue_2) (.z _returnvalue_2)) _lerp_forward) false false))
    (:Finished
      (Collision|SetCollisionResponsetoChannel (Variables|Default|GetCapsuleComponent) "ECC_WorldDynamic" "ECR_Block"))))

(event EventBeginPlay
  (bind _bpcomp_dialogue (Variables|Default|GetBPComp_Dialogue))
  (Variables|Default|SetAnim_Sitting true)
  (Variables|/Game/Billy/DialogueSystemMKII/BPComp_Dialogue.BPComp_Dialogue_C|SetActorToTrigger1 _bpcomp_dialogue (Variables|Default|GetDialogueTriggerObject1))
  (Variables|/Game/Billy/DialogueSystemMKII/BPComp_Dialogue.BPComp_Dialogue_C|SetActorToTrigger2 _bpcomp_dialogue (Variables|Default|GetDialogueTriggerObject2))
  (Variables|/Game/Billy/DialogueSystemMKII/BPComp_Dialogue.BPComp_Dialogue_C|SetActorToTrigger3 _bpcomp_dialogue (Variables|Default|GetDialogueTriggerObject3))
  (Variables|/Game/Billy/DialogueSystemMKII/BPComp_Dialogue.BPComp_Dialogue_C|SetActorToTrigger4 _bpcomp_dialogue (Variables|Default|GetDialogueTriggerObject4))
  (Variables|/Game/Billy/DialogueSystemMKII/BPComp_Dialogue.BPComp_Dialogue_C|SetActorToTrigger5 _bpcomp_dialogue (Variables|Default|GetDialogueTriggerObject5))
  (bind _asgi_hero_adrift (Utilities|Casting|CastToGI_HeroAdrift (Game|GetGameInstance)))
  (if (.Value (Utilities|Map|Find (Variables|/Game/Ash/Blueprints/GI_HeroAdrift.GI_HeroAdrift_C|GetWizardIslandProgress _asgi_hero_adrift) "RangarLeft"))
    (Variables|/Game/Billy/DialogueSystemMKII/BPComp_Dialogue.BPComp_Dialogue_C|SetDialogueTree (Variables|Default|GetBPComp_Dialogue) "/Game/Ash/Blueprints/LevelSpecific/IsleOfTheForetold/BT_KeratosMonologue.BT_KeratosMonologue")
    (else
      (Variables|/Game/Billy/DialogueSystemMKII/BPComp_Dialogue.BPComp_Dialogue_C|SetDialogueTree (Variables|Default|GetBPComp_Dialogue) "/Game/Ash/Blueprints/LevelSpecific/IsleOfTheForetold/BT_KeratosMonologueShort.BT_KeratosMonologueShort"))))

(fn ConstructionScript
  (|CallParentFunction))