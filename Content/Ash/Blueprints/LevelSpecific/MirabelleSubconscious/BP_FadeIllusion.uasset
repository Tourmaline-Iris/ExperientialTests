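; Interactable in the Mirabelle subconscious level that fades out a linked illusion actor and darkens its cloud and fog.
; BeginPlay creates dynamic materials for the illusion's static and skeletal meshes and the cloud.
; OnInteract ignores a trace channel on those meshes, then a timeline drives dither and lerps colours towards dark grey.
; On finish it reports to BP_FadeIllusionFinal, which may show the final illusion, then destroys itself and, via EndPlay, the illusion.
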(event EventBeginPlay
  (for _array_element (Actor|GetComponentsByClass (Variables|Default|GetIllusionToFade) "/Script/Engine.StaticMeshComponent")
    (for (_array_element_2 _array_index) (Rendering|Material|GetMaterials _array_element)
      (bind _returnvalue (Rendering|Material|CreateDynamicMaterialInstance _array_element_2 "None" "None" :!class /Script/Engine.KismetMaterialLibrary))
      (Utilities|Array|Add (Variables|Default|GetIllusionDynamicMaterials) _returnvalue)
      (Rendering|Material|SetMaterial _array_element _array_index _returnvalue)))
  (for _array_element_3 (Actor|GetComponentsByClass (Variables|Default|GetIllusionToFade) "/Script/Engine.SkeletalMeshComponent")
    (for (_array_element_4 _array_index_2) (Rendering|Material|GetMaterials _array_element_3)
      (bind _returnvalue_2 (Rendering|Material|CreateDynamicMaterialInstance _array_element_4 "None" "None" :!class /Script/Engine.KismetMaterialLibrary))
      (Utilities|Array|Add (Variables|Default|GetIllusionDynamicMaterials) _returnvalue_2)
      (Rendering|Material|SetMaterial _array_element_3 _array_index_2 _returnvalue_2)))
  (bind _returnvalue_3 (Rendering|Material|CreateDynamicMaterialInstance (Rendering|Material|GetMaterial (Variables|/Script/Engine.StaticMeshActor|GetStaticMeshComponent (Variables|Default|GetCloudToDarken)) 0) "None" "None" :!class /Script/Engine.KismetMaterialLibrary))
  (bind _output_get (Variables|Default|SetCloudDynamicMaterial _returnvalue_3))
  (Rendering|Material|SetMaterial (Variables|/Script/Engine.StaticMeshActor|GetStaticMeshComponent (Variables|Default|GetCloudToDarken)) 0 _output_get))

(event EventOnInteract
  (params (Interactor :type First%20Person%20Character%20Object%20Reference))
  (bind _illusiontofade (Variables|Default|GetIllusionToFade))
  (for _array_element (Actor|GetComponentsByClass _illusiontofade "/Script/Engine.StaticMeshComponent")
    (Utilities|IsValid _array_element
      (:Is%20Valid
        (Collision|SetCollisionResponsetoChannel _array_element "ECC_GameTraceChannel3" "ECR_Ignore"))))
  (for _array_element_2 (Actor|GetComponentsByClass _illusiontofade "/Script/Engine.SkeletalMeshComponent")
    (Utilities|IsValid _array_element_2
      (:Is%20Valid
        (Collision|SetCollisionResponsetoChannel _array_element_2 "ECC_GameTraceChannel3" "ECR_Ignore"))))
  (bind (_direction _fadeillusion _darkencloud) (Timeline|FadeIllusion PlayFromStart)
    (:Update
      (for _array_element_3 (Variables|Default|GetIllusionDynamicMaterials)
        (Rendering|Material|SetScalarParameterValue _array_element_3 "DitherPercent" _fadeillusion :!class /Script/Engine.MaterialInstanceDynamic))
      (bind _returnvalue (Rendering|Material|GetVectorParameterValue (Variables|Default|GetCloudDynamicMaterial) "Colour" :!class /Script/Engine.MaterialInstanceDynamic))
      (Rendering|Material|SetVectorParameterValue (Variables|Default|GetCloudDynamicMaterial) "Colour" (Math|Color|Lerp(LinearColor) _returnvalue "(R=0.078125,G=0.078125,B=0.078125,A=1.000000)" _darkencloud) :!class /Script/Engine.MaterialInstanceDynamic)
      (Effects|Components|ParticleSystem|SetColorParameter (Variables|/Script/Engine.Emitter|GetParticleSystemComponent (Variables|Default|GetFog)) "Colour" (Math|Color|Lerp(LinearColor) _returnvalue "(R=0.078125,G=0.078125,B=0.078125,A=1.000000)" _darkencloud)))
    (:Finished
      (bind _asbp_fade_illusion_final (Utilities|Casting|CastToBP_FadeIllusionFinal (Variables|Default|GetIllusionFadeFinal)))
      (bind _returnvalue_2 (Default|AddIllusionFaded _asbp_fade_illusion_final))
      (if _returnvalue_2
        (Default|ShowIllusion _asbp_fade_illusion_final))
      (Rendering|SetActorHiddenInGame (Variables|Default|GetIllusionToFade) true)
      (Actor|DestroyActor))))

(event EventEndPlay
  (params (EndPlayReason :type EEndPlayReason%20Enum :default "Destroyed"))
  (Actor|DestroyActor (Variables|Default|GetIllusionToFade)))

(fn ConstructionScript)