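; BP_Fruit is a one-time banana bundle pickup on Pirate Island that becomes interactable once the player meets Mango.
; The MetMangoTrigger event switches the mesh's custom trace channel response to Block to enable interaction.
; Interacting notifies BP_FruitBasket, saves PlayerHasFruit to the GI_HeroAdrift progress map and destroys the actor.
; On BeginPlay, it destroys itself if that saved flag is already set.
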(event Custom|EnableInteraction
  (Collision|SetCollisionResponsetoChannel (Variables|Default|GetSM_MERGED_banana_bundle) "ECC_GameTraceChannel3" "ECR_Block"))

(event EventBeginPlay
  (EventDispatchers|BindEventtoPlayerMetMango (Variables|Default|GetMetMangoTrigger) (delegate Custom|EnableInteraction))
  (bind _asgi_hero_adrift (Utilities|Casting|CastToGI_HeroAdrift (Game|GetGameInstance)))
  (if (.Value (Utilities|Map|Find (Variables|/Game/Ash/Blueprints/GI_HeroAdrift.GI_HeroAdrift_C|GetPirateIslandProgress _asgi_hero_adrift) "PlayerHasFruit"))
    (Actor|DestroyActor)))

(event EventOnInteract
  (params (Interactor :type First%20Person%20Character%20Object%20Reference))
  (bind _asbp_fruit_basket (Utilities|Casting|CastToBP_FruitBasket (Variables|Default|GetFruitBasket)))
  (Default|PlayerPicksUpFruit _asbp_fruit_basket)
  (bind _asgi_hero_adrift (Utilities|Casting|CastToGI_HeroAdrift (Game|GetGameInstance)))
  (Default|SaveLevelProgress _asgi_hero_adrift (Variables|/Game/Ash/Blueprints/GI_HeroAdrift.GI_HeroAdrift_C|GetPirateIslandProgress _asgi_hero_adrift) "PlayerHasFruit")
  (Actor|DestroyActor))

(fn ConstructionScript)