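; Secondary anchor weapon for the first-person player that throws an anchor on a chain and can pull targets in.
; Secondary use spawns a camera-aimed BP_AnchorProjectile, hides the weapon mesh and attaches a runtime cable to the projectile, undone when it returns.
; PullOther uses a timeline to lerp the target to the player's secondary grip socket.
; Tick traces from the camera for "Hookable" actors to switch the HUD's secondary icon.
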(event Custom|ProjectileReturned
  (bind _chain (Variables|Default|GetChain))
  (Utilities|IsValid _chain
    (:Is%20Valid
      (Components|DestroyComponent _chain))
    (:Is%20Not%20Valid
      _))
  (Rendering|SetVisibility (Variables|Default|GetStaticMesh) true false))

(event Custom|PullOther
  (params (Other :type Scene%20Component%20Object%20Reference) (PlayerSkeletalMesh :type Scene%20Component%20Object%20Reference))
  (bind _pulltrack (Timeline|Pull PlayFromStart)
    (:Update
      (Transformation|SetWorldLocation Other (Math|Vector|Lerp(Vector) (Transformation|GetWorldLocation Other) (Transformation|GetSocketLocation PlayerSkeletalMesh "GripPointSecondary") _pulltrack) false false))))

(event EventTick
  (params (DeltaSeconds :type Float%20%28single-precision%29))
  (bind _firstpersoncamera (Variables|Default|GetFirstPersonCamera))
  (bind _returnvalue (Transformation|GetWorldLocation _firstpersoncamera))
  (bind _outhit (Collision|LineTraceByChannel _returnvalue (+ _returnvalue (* (Math|Vector|GetForwardVector (Transformation|GetWorldRotation _firstpersoncamera)) (Variables|Default|GetRange))) "TraceTypeQuery1" false 0 "None" true "(R=1.000000,G=0.000000,B=0.000000,A=1.000000)" "(R=0.000000,G=1.000000,B=0.000000,A=1.000000)" DeltaSeconds))
  (Utilities|IsValid (.HitActor (Collision|BreakHitResult _outhit))
    (:Is%20Valid
      (if (Actor|ActorHasTag (.HitActor (Collision|BreakHitResult _outhit)) "Hookable")
        (Variables|Default|SetEnumSecondaryIcon "NewEnumerator1")
        (else
          (Variables|Default|SetEnumSecondaryIcon "NewEnumerator0" :!label _label))))
    (:Is%20Not%20Valid
      (goto _label)))
  (Default|SecondaryWeaponTick (Variables|Default|GetGameplay%20HUD) (Variables|Default|GetEnumSecondaryIcon)))

(event EventBeginPlay
  (|CallParentFunction))

(event EventEndPlay
  (params (EndPlayReason :type EEndPlayReason%20Enum :default "Destroyed"))
  (bind _output_get (Variables|Default|SetEnumSecondaryIcon "NewEnumerator0"))
  (Default|SecondaryWeaponTick (Variables|Default|GetGameplay%20HUD) _output_get))

(event EventUseSecondary
  (params (Instigator :type Pawn%20Object%20Reference))
  (bind _staticmesh (Variables|Default|GetStaticMesh))
  (bind _returnvalue (Transformation|GetWorldTransform _staticmesh))
  (|CallParentFunction Instigator)
  (bind _asfirst_person_character (Utilities|Casting|CastToFirstPersonCharacter Instigator))
  (bind _spawntransform (CallFunction|AimProjectile (Variables|/Game/FirstPersonBP/Blueprints/FirstPersonCharacter.FirstPersonCharacter_C|GetFirstPersonCamera _asfirst_person_character) (Transformation|GetWorldLocation (Variables|Default|GetStaticMesh)) (Variables|Default|GetRange)))
  (bind _returnvalue_2 (Game|SpawnActorfromClass "/Game/Ash/Blueprints/Player/BP_AnchorProjectile.BP_AnchorProjectile_C" _spawntransform "Undefined" self (Variables|/Game/FirstPersonBP/Blueprints/FirstPersonCharacter.FirstPersonCharacter_C|GetSkeletalMesh _asfirst_person_character) 0.2 _asfirst_person_character))
  (Rendering|SetVisibility _staticmesh false false)
  (bind _returnvalue_3 (AddComponent|AddCableComponent true (Math|Transform|MakeTransform (.location _returnvalue) (.rotation _returnvalue) "1,1,1")))
  (bind _output_get (Variables|Default|SetChain _returnvalue_3))
  (Class|CableComponent|SetAttachEndto _output_get _returnvalue_2 "None" "None"))

(fn ConstructionScript)