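; Base Blueprint for secondary weapons, providing a shared use event and a projectile aiming helper.
; UseSecondary takes an Instigator and is an empty event here.
; AimProjectile traces on the Visibility channel along the player camera's forward vector, then returns a transform at the spawn location rotated toward the hit point, or the trace end on a miss, so projectiles converge on the camera's aim point.
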(event Custom|UseSecondary
  (params (Instigator :type Pawn%20Object%20Reference)))

(fn ConstructionScript)

(fn AimProjectile
  (params (PlayerCamera :type Camera%20Component%20Object%20Reference) (SpawnLocation :type Vector) (LineTraceRange :type Float%20%28single-precision%29))
  (bind _returnvalue (Transformation|GetWorldLocation PlayerCamera))
  (bind (_outhit _returnvalue_2) (Collision|LineTraceByChannel _returnvalue (+ _returnvalue (* (Math|Vector|GetForwardVector (Transformation|GetWorldRotation PlayerCamera)) LineTraceRange)) "TraceTypeQuery1" false 0 "None" true "(R=1.000000,G=0.000000,B=0.000000,A=1.000000)" "(R=0.000000,G=1.000000,B=0.000000,A=1.000000)" (Utilities|Time|GetWorldDeltaSeconds)))
  (return (Math|Transform|MakeTransform SpawnLocation (Math|Rotator|FindLookatRotation SpawnLocation (Math|Vector|SelectVector (.ImpactPoint (Collision|BreakHitResult _outhit)) (.TraceEnd (Collision|BreakHitResult _outhit)) _returnvalue_2)))))