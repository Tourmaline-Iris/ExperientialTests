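; BP_Hook is a hook projectile that flies out at a configurable speed, returns to the player's secondary grip socket and pulls whatever it hits along.
; It ignores the instigator's capsule.
; After a short delay or on a hit, the Return timeline stops movement and lerps the mesh back, while MoveOther drags the hit actor's root.
; When Return finishes, it resets the player's secondary weapon with FireRate and destroys itself.
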(event OnComponentHit(SphereCollider)
  (params (HitComponent :type Primitive%20Component%20Object%20Reference) (OtherActor :type Actor%20Object%20Reference) (OtherComp :type Primitive%20Component%20Object%20Reference) (NormalImpulse :type Vector :default "0, 0, 0") (Hit :type Hit%20Result%20Structure%20%28by%20ref%29))
  (Utilities|FlowControl|Sequence
    (:then_0
      (bind _returntrack (Timeline|Return Play)
        (:Update
          (Variables|/Script/Engine.MovementComponent|SetVelocity (Variables|Default|GetProjectileMovement) "0, 0, 0")
          (Transformation|SetWorldLocation (Variables|Default|GetMesh) (Math|Vector|Lerp(Vector) (Transformation|GetWorldLocation (Variables|Default|GetMesh)) (Transformation|GetSocketLocation (Variables|Default|GetPlayerSkeletalMesh) "GripPointSecondary") _returntrack) false false))
        (:Finished
          (bind _asfirst_person_character (Utilities|Casting|CastToFirstPersonCharacter (Game|GetPlayerCharacter 0)))
          (Default|ResetSecondaryWeapon _asfirst_person_character (Variables|Default|GetFireRate))
          (Actor|DestroyActor))))
    (:then_1
      (bind _returntrack_2 (Timeline|MoveOther Play)
        (:Update
          (Transformation|SetWorldLocation (Variables|/Script/Engine.Actor|GetRootComponent OtherActor) (Math|Vector|Lerp(Vector) (Transformation|GetWorldLocation (Variables|/Script/Engine.Actor|GetRootComponent OtherActor)) (Transformation|GetSocketLocation (Variables|Default|GetPlayerSkeletalMesh) "GripPointSecondary") _returntrack_2) false false))))))

(event EventBeginPlay
  (bind _asfirst_person_character (Utilities|Casting|CastToFirstPersonCharacter (Game|GetInstigator)))
  (Class|PrimitiveComponent|IgnoreComponentwhenMoving (Variables|Default|GetSphereCollider) (Variables|/Script/Engine.Character|GetCapsuleComponent _asfirst_person_character) true)
  (Utilities|FlowControl|Delay 0.2)
  (bind _returntrack (Timeline|Return Play)
    (:Update
      (Variables|/Script/Engine.MovementComponent|SetVelocity (Variables|Default|GetProjectileMovement) "0, 0, 0")
      (Transformation|SetWorldLocation (Variables|Default|GetMesh) (Math|Vector|Lerp(Vector) (Transformation|GetWorldLocation (Variables|Default|GetMesh)) (Transformation|GetSocketLocation (Variables|Default|GetPlayerSkeletalMesh) "GripPointSecondary") _returntrack) false false))
    (:Finished
      (bind _asfirst_person_character_2 (Utilities|Casting|CastToFirstPersonCharacter (Game|GetPlayerCharacter 0)))
      (Default|ResetSecondaryWeapon _asfirst_person_character_2 (Variables|Default|GetFireRate))
      (Actor|DestroyActor))))

(fn ConstructionScript
  (bind _projectilemovement (Variables|Default|GetProjectileMovement))
  (bind _hookvelocity (Variables|Default|GetHookVelocity))
  (Variables|/Script/Engine.ProjectileMovementComponent|SetMaxSpeed _projectilemovement _hookvelocity)
  (Variables|/Script/Engine.ProjectileMovementComponent|SetInitialSpeed _projectilemovement _hookvelocity)
  (Variables|/Script/Engine.MovementComponent|SetVelocity _projectilemovement (Math|Vector|MakeVector _hookvelocity 0.0 0.0)))