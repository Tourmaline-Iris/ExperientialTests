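; Handler for Aria's druid island that sets the level layout and Aria's dialogue from the player's quest progress.
; On BeginPlay it finds the first unfinished entry in the GameInstance's DruidIslandProgress map and derives a visibility array and Aria index.
; It toggles visibility and collision on grouped attached actors, swaps the active Aria and assigns her dialogue tree.
; Talkable plants appear only when the player has the talk-to-plants flag.
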(event EventLoadPlants
  (bind _plantscontainer (Variables|Default|GetPlantsContainer))
  (bind _outactors (Actor|GetAttachedActors _plantscontainer true))
  (if (Variables|/Game/Ash/Blueprints/GI_HeroAdrift.GI_HeroAdrift_C|GetPlayerHasTalkToPlants (.AsGI%20Hero%20Adrift (Utilities|Casting|CastToGI_HeroAdrift (Game|GetGameInstance))))
    (for _array_element _outactors
      (Rendering|SetActorHiddenInGame _array_element false)
      (bind _asbp_plant_talkable (Utilities|Casting|CastToBP_PlantTalkable _array_element))
      (Collision|SetCollisionResponsetoChannel (Variables|/Game/Billy/DialogueSystemMKII/BP_PlantTalkable.BP_PlantTalkable_C|GetSphere _asbp_plant_talkable) "ECC_GameTraceChannel3" "ECR_Block"))
    (else
      (for _array_element_2 _outactors
        (Rendering|SetActorHiddenInGame _array_element_2 true)
        (bind _asbp_plant_talkable_2 (Utilities|Casting|CastToBP_PlantTalkable _array_element_2))
        (Collision|SetCollisionResponsetoChannel (Variables|/Game/Billy/DialogueSystemMKII/BP_PlantTalkable.BP_PlantTalkable_C|GetSphere _asbp_plant_talkable_2) "ECC_GameTraceChannel3" "ECR_Ignore")))))

(event EventUpdateLevelProgress
  (bind (_progressindex _arrayhasfalse) (CallFunction|GetProgress))
  (if _arrayhasfalse
    (bind _result (Math|Integer|DecrementInt _progressindex)
      (:%20%20
        (CallFunction|SetAriaDialogue _result (not _arrayhasfalse))
        (switch int _result
          (:Default
            (Variables|Default|SetObjectStateArray (Utilities|Array|MakeArray false false true true true))
            (Variables|Default|SetAriaIndex 0)
            (bind _values (Utilities|Map|Values (Variables|Default|GetObjectsToChange) :!label _label))
            (CallFunction|SetObjectsVisibility (Variables|Default|GetObjectStateArray) _values))
          (:0
            (CallFunction|LoadPlants)
            (Variables|Default|SetObjectStateArray (Utilities|Array|MakeArray false false true true true))
            (Variables|Default|SetAriaIndex 0 :!label _label_2)
            (goto _label))
          (:1
            (Variables|Default|SetObjectStateArray (Utilities|Array|MakeArray true false true true true))
            (goto _label_2))
          (:2
            (Variables|Default|SetObjectStateArray (Utilities|Array|MakeArray true true false true true) :!label _label_3)
            (Variables|Default|SetAriaIndex 1 :!label _label_4))
          (:3
            (goto _label_3))
          (:4
            (Variables|Default|SetObjectStateArray (Utilities|Array|MakeArray true true true false true))
            (goto _label_4))
          (:5
            (Variables|Default|SetObjectStateArray (Utilities|Array|MakeArray true true true true false) :!label _label_5)
            (goto _label_4)))))
    (else
      (goto _label_5))))

(event EventChangeLayoutonEntry
  (bind _values (Utilities|Map|Values (Variables|Default|GetObjectsToChange)))
  (CallFunction|SetObjectsVisibility (Variables|Default|GetObjectStateArray) _values)
  (CallFunction|SetCurrentAria (Variables|Default|GetAriaIndex))
  (bind (_progressindex _arrayhasfalse) (CallFunction|GetProgress))
  (bind _result (Math|Integer|DecrementInt _progressindex)
    (:%20%20
      (CallFunction|SetAriaDialogue _result (not _arrayhasfalse)))))

(event EventBeginPlay
  (CallFunction|LoadPlants)
  (CallFunction|UpdateLevelProgress)
  (CallFunction|ChangeLayoutonEntry))

(fn ConstructionScript)

(fn SetObjectsVisibility
  (params (IsHidden :type Array%20of%20Booleans) (Objects :type Array%20of%20Actor%20Object%20References))
  (for (_array_element _array_index) Objects
    (for _array_element_2 (Actor|GetAttachedActors _array_element true)
      (Rendering|SetActorHiddenInGame _array_element_2 (Utilities|Array|Get(acopy) IsHidden _array_index))
      (Collision|SetActorEnableCollision _array_element_2 (not (Utilities|Array|Get(acopy) IsHidden _array_index))))))

(fn SetAriaDialogue
  (params (DialogueIndex :type Integer) (IsFinished :type Boolean))
  (if IsFinished
    (Variables|/Game/Billy/DialogueSystemMKII/BPComp_Dialogue.BPComp_Dialogue_C|SetDialogueTree (Variables|/Game/Billy/DialogueSystemMKII/BP_SkeletalMeshDialogue.BP_SkeletalMeshDialogue_C|GetBPComp_Dialogue (Variables|Default|GetCurrentAria)) (Utilities|Array|Get(acopy) (Variables|Default|GetAriaDialogues) 5))
    (elif (>= DialogueIndex 0)
      (Variables|/Game/Billy/DialogueSystemMKII/BPComp_Dialogue.BPComp_Dialogue_C|SetDialogueTree (Variables|/Game/Billy/DialogueSystemMKII/BP_SkeletalMeshDialogue.BP_SkeletalMeshDialogue_C|GetBPComp_Dialogue (Variables|Default|GetCurrentAria)) (Utilities|Array|Get(acopy) (Variables|Default|GetAriaDialogues) DialogueIndex)))))

(fn SetCurrentAria
  (params (AriaIndex :type Integer))
  (bind _ariaarray (Variables|Default|GetAriaArray))
  (bind _output (Utilities|Array|Get(acopy) _ariaarray AriaIndex))
  (bind _capsulecomponent (Variables|/Script/Engine.Character|GetCapsuleComponent _output))
  (for _array_element (Variables|Default|GetAriaArray)
    (Rendering|SetActorHiddenInGame _array_element true)
    (Collision|SetCollisionResponsetoChannel (Variables|/Script/Engine.Character|GetCapsuleComponent _array_element) "ECC_GameTraceChannel3" "ECR_Ignore")
    (Collision|SetCollisionResponsetoChannel (Variables|/Script/Engine.Character|GetCapsuleComponent _array_element) "ECC_Pawn" "ECR_Ignore")
    (Collision|SetCollisionResponsetoChannel (Variables|/Script/Engine.Character|GetCapsuleComponent _array_element) "ECC_GameTraceChannel1" "ECR_Ignore"))
  (Variables|Default|SetCurrentAria _output)
  (Rendering|SetActorHiddenInGame _output false)
  (Collision|SetCollisionResponsetoChannel _capsulecomponent "ECC_GameTraceChannel3" "ECR_Block")
  (Collision|SetCollisionResponsetoChannel _capsulecomponent "ECC_Pawn" "ECR_Block")
  (Collision|SetCollisionResponsetoChannel _capsulecomponent "ECC_GameTraceChannel1" "ECR_Block"))

(fn GetProgress
  (bind _values (Utilities|Map|Values (Variables|/Game/Ash/Blueprints/GI_HeroAdrift.GI_HeroAdrift_C|GetDruidIslandProgress (.AsGI%20Hero%20Adrift (Utilities|Casting|CastToGI_HeroAdrift (Game|GetGameInstance))))))
  (return (Utilities|Array|FindItem _values false) (Utilities|Array|ContainsItem _values false)))