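; BP_HealthPickup is a health pickup actor that pops upward on spawn and heals the player on overlap.
; BeginPlay launches GroundSphere with an impulse, raises PickupSphere via MoveComponentTo, and runs a timeline driving the mesh's yaw spin.
; Tick keeps the static mesh at PickupSphere's location with a swept move.
; The first player overlap adds HealAmount to the FirstPersonCharacter's HealthComponent, clamped to MaxHealth, then destroys the pickup.
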(event OnComponentBeginOverlap(PickupSphere)
  (params (OverlappedComponent :type Primitive%20Component%20Object%20Reference) (OtherActor :type Actor%20Object%20Reference) (OtherComp :type Primitive%20Component%20Object%20Reference) (OtherBodyIndex :type Integer) (bFromSweep :type Boolean) (SweepResult :type Hit%20Result%20Structure%20%28by%20ref%29))
  (bind _returnvalue (Game|GetPlayerCharacter 0))
  (if (== OtherActor _returnvalue)
    (Utilities|FlowControl|DoOnce false
      (:Completed
        (bind _asfirst_person_character (Utilities|Casting|CastToFirstPersonCharacter _returnvalue))
        (Variables|/Game/Ash/Blueprints/Components/HealthComponent.HealthComponent_C|SetCurrentHealth (Variables|/Game/FirstPersonBP/Blueprints/FirstPersonCharacter.FirstPersonCharacter_C|GetHealthComponent _asfirst_person_character) (Math|Float|Clamp(Float) (+ (Variables|/Game/Ash/Blueprints/Components/HealthComponent.HealthComponent_C|GetCurrentHealth (Variables|/Game/FirstPersonBP/Blueprints/FirstPersonCharacter.FirstPersonCharacter_C|GetHealthComponent _asfirst_person_character)) (Variables|Default|GetHealAmount)) 0.0 (Variables|/Game/Ash/Blueprints/Components/HealthComponent.HealthComponent_C|GetMaxHealth (Variables|/Game/FirstPersonBP/Blueprints/FirstPersonCharacter.FirstPersonCharacter_C|GetHealthComponent _asfirst_person_character))))
        (Actor|DestroyActor)))))

(event EventBeginPlay
  (Physics|AddImpulse (Variables|Default|GetGroundSphere) "0.000000,0.000000,700.000000" "None" true)
  (Components|MoveComponentTo (Variables|Default|GetPickupSphere) "0, 0,70.000000" "0, 0, 0" false false (Variables|Default|GetTimeToApex) false)
  (Components|Timeline|SetPlayRate (Variables|Default|GetMeshRotationSpeed) (Variables|Default|GetTimeToApex))
  (bind _rotationratez (Timeline|MeshRotationSpeed PlayFromStart)
    (:Update
      (Variables|/Script/Engine.RotatingMovementComponent|SetRotationRate (Variables|Default|GetRotatingMovement) (Math|Rotator|MakeRotator 0.0 0.0 _rotationratez)))))

(event EventTick
  (params (DeltaSeconds :type Float%20%28single-precision%29))
  (bind _staticmesh (Variables|Default|GetStaticMesh))
  (bind _pickupsphere (Variables|Default|GetPickupSphere))
  (bind _returnvalue (Transformation|GetWorldLocation _pickupsphere))
  (if (Math|Vector|NotEqual(Vector) (Transformation|GetWorldLocation _staticmesh) _returnvalue 0.0001)
    (Transformation|SetWorldLocation _staticmesh _returnvalue true false)))

(fn ConstructionScript)