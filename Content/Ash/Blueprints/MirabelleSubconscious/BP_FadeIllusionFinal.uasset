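; Interactable actor for the final illusion in Mirabelle's subconscious, which dithers a linked illusion actor in and later fades it out.
; BeginPlay hides the illusion and creates dynamic materials for its meshes and assigned clouds.
; ShowIllusion drives a DitherPercent timeline, then enables collision; OnInteract broadcasts EndDenial, fades the illusion, darkens cloud colours and destroys itself.
; AddIllusionFaded counts faded illusions and reports when the required number is reached.
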(event Custom|ShowIllusion
  (Rendering|SetActorHiddenInGame (Variables|Default|GetIllusionToFade) false)
  (bind _ditherpercent (Timeline|Show Play)
    (:Update
      (for _array_element (Variables|Default|GetIllusionDynamicMaterials)
        (Rendering|Material|SetScalarParameterValue _array_element "DitherPercent" _ditherpercent :!class /Script/Engine.MaterialInstanceDynamic)))
    (:Finished
      (Collision|SetActorEnableCollision (Variables|Default|GetIllusionToFade) true))))

(event EventBeginPlay
  (bind _illusiontofade (Variables|Default|GetIllusionToFade))
  (Rendering|SetActorHiddenInGame _illusiontofade true)
  (Collision|SetActorEnableCollision _illusiontofade false)
  (for _array_element (Actor|GetComponentsByClass (Variables|Default|GetIllusionToFade) "/Script/Engine.StaticMeshComponent")
    (for (_array_element_2 _array_index) (Rendering|Material|GetMaterials _array_element)
      (bind _returnvalue (Rendering|Material|CreateDynamicMaterialInstance _array_element_2 "None" "None" :!class /Script/Engine.KismetMaterialLibrary))
      (Utilities|Array|Add (Variables|Default|GetIllusionDynamicMaterials) _returnvalue)
      (Rendering|Material|SetMaterial _array_element _array_index _returnvalue)))
  (for _array_element_3 (Actor|GetComponentsByClass (Variables|Default|GetIllusionToFade) "/Script/Engine.SkeletalMeshComponent")
    (for (_array_element_4 _array_index_2) (Rendering|Material|GetMaterials _array_element_3)
      (bind _returnvalue_2 (Rendering|Material|CreateDynamicMaterialInstance _array_element_4 "None" "None" :!class /Script/Engine.KismetMaterialLibrary))
      (Utilities|Array|Add (Variables|Default|GetIllusionDynamicMaterials) _returnvalue_2)
      (Rendering|Material|SetMaterial _array_element_3 _array_index_2 _returnvalue_2))
    (for _array_element_5 (Variables|Default|GetCloudsToDarken)
      (bind _returnvalue_3 (Rendering|Material|CreateDynamicMaterialInstance (Rendering|Material|GetMaterial (Variables|/Script/Engine.StaticMeshActor|GetStaticMeshComponent _array_element_5) 0) "None" "None" :!class /Script/Engine.KismetMaterialLibrary))
      (bind _returnvalue_4 (Utilities|Array|Add (Variables|Default|GetCloudDynamicMaterials) _returnvalue_3))
      (Rendering|Material|SetMaterial (Variables|/Script/Engine.StaticMeshActor|GetStaticMeshComponent _array_element_5) _returnvalue_4 _returnvalue_3))
    (for _array_element_6 (Variables|Default|GetIllusionDynamicMaterials)
      (Rendering|Material|SetScalarParameterValue _array_element_6 "DitherPercent" 0.0 :!class /Script/Engine.MaterialInstanceDynamic))))

(event EventOnInteract
  (params (Interactor :type First%20Person%20Character%20Object%20Reference))
  (Default|CallEndDenial)
  (bind (_direction _fadeillusion _darkencloud) (Timeline|FadeIllusion PlayFromStart)
    (:Update
      (for _array_element (Variables|Default|GetIllusionDynamicMaterials)
        (Rendering|Material|SetScalarParameterValue _array_element "DitherPercent" _fadeillusion :!class /Script/Engine.MaterialInstanceDynamic))
      (for _array_element_2 (Variables|Default|GetCloudDynamicMaterials)
        (bind _returnvalue (Rendering|Material|GetVectorParameterValue _array_element_2 "Colour" :!class /Script/Engine.MaterialInstanceDynamic))
        (Rendering|Material|SetVectorParameterValue _array_element_2 "Colour" (Math|Color|Lerp(LinearColor) _returnvalue "(R=0.078125,G=0.078125,B=0.078125,A=1.000000)" _darkencloud) :!class /Script/Engine.MaterialInstanceDynamic)))
    (:Finished
      (Rendering|SetActorHiddenInGame (Variables|Default|GetIllusionToFade) true)
      (Actor|DestroyActor))))

(event EventEndPlay
  (params (EndPlayReason :type EEndPlayReason%20Enum :default "Destroyed"))
  (Actor|DestroyActor (Variables|Default|GetIllusionToFade)))

(fn ConstructionScript)

(fn AddIllusionFaded
  (bind _output_get (Variables|Default|SetIllusionsFaded (+ (Variables|Default|GetIllusionsFaded) 1)))
  (return (>= _output_get (Variables|Default|GetRequiredIllusions))))