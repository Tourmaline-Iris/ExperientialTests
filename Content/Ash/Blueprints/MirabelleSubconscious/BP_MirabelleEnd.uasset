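; BP_MirabelleEnd is an interactable ending actor in Mirabelle's subconscious that returns the player to LVL_PirateIsland at the MangoBed player start.
; On BeginPlay it creates dynamic materials for the hidden Mango static mesh and every skeletal mesh slot.
; Interacting reveals Mango with a timeline-driven dither fade, pauses, then dither-fades both meshes out, hides them and opens the level.
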(event EventOnInteract
  (params (Interactor :type First%20Person%20Character%20Object%20Reference))
  (Rendering|SetVisibility (Variables|Default|GetStaticMesh) true false)
  (bind _ditherpercent (Timeline|FadeIn PlayFromStart)
    (:Update
      (Rendering|Material|SetScalarParameterValue (Variables|Default|GetMangoDynamicMaterial) "DitherPercent" _ditherpercent :!class /Script/Engine.MaterialInstanceDynamic))
    (:Finished
      (Utilities|FlowControl|Delay 2.0)
      (bind _ditherpercent_2 (Timeline|FadeOut PlayFromStart)
        (:Update
          (Rendering|Material|SetScalarParameterValue (Variables|Default|GetMangoDynamicMaterial) "DitherPercent" _ditherpercent_2 :!class /Script/Engine.MaterialInstanceDynamic)
          (for _array_element (Variables|Default|GetMirabelleDynamicMaterials)
            (Rendering|Material|SetScalarParameterValue _array_element "DitherPercent" _ditherpercent_2 :!class /Script/Engine.MaterialInstanceDynamic)))
        (:Finished
          (Rendering|SetVisibility (Variables|Default|GetStaticMesh) false false)
          (Rendering|SetVisibility (Variables|Default|GetSkeletalMesh) false false)
          (Utilities|FlowControl|Delay 1.0)
          (bind _output_get (Variables|Default|SetPlayerStartTag "MangoBed"))
          (Game|OpenLevel(byObjectReference) "/Game/Ash/Levels/LVL_PirateIsland.LVL_PirateIsland" true _output_get))))))

(event EventBeginPlay
  (bind _returnvalue (Rendering|Material|CreateDynamicMaterialInstance (Rendering|Material|GetMaterial (Variables|Default|GetStaticMesh) 0) "None" "None" :!class /Script/Engine.KismetMaterialLibrary))
  (bind _output_get (Variables|Default|SetMangoDynamicMaterial _returnvalue))
  (Rendering|Material|SetMaterial (Variables|Default|GetStaticMesh) 0 _output_get)
  (Rendering|Material|SetScalarParameterValue (Variables|Default|GetMangoDynamicMaterial) "DitherPercent" 0.0 :!class /Script/Engine.MaterialInstanceDynamic)
  (Rendering|SetVisibility (Variables|Default|GetStaticMesh) false false)
  (for _array_element (Rendering|Material|GetMaterials (Variables|Default|GetSkeletalMesh))
    (bind _returnvalue_2 (Rendering|Material|CreateDynamicMaterialInstance _array_element "None" "None" :!class /Script/Engine.KismetMaterialLibrary))
    (bind _returnvalue_3 (Utilities|Array|Add (Variables|Default|GetMirabelleDynamicMaterials) _returnvalue_2))
    (Rendering|Material|SetMaterial (Variables|Default|GetSkeletalMesh) _returnvalue_3 _returnvalue_2)))

(fn ConstructionScript)