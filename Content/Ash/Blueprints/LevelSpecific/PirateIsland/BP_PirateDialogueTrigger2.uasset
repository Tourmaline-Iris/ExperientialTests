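; Dialogue trigger for Pirate Island that applies the gameplay results of talking to Mango, selected by a function enum.
; On interact, the fruit stage flags Mango to give an item, restores player health to maximum and advances to the help stage.
; The help stage swaps Mango's dialogue tree to bedroom directions, saves "AskedToHelp" progress and enables a collision channel on the bed.
; BeginPlay selects the help stage if that progress is saved.
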(event EventBeginPlay
  (bind _asgi_hero_adrift (Utilities|Casting|CastToGI_HeroAdrift (Game|GetGameInstance)))
  (if (.Value (Utilities|Map|Find (Variables|/Game/Ash/Blueprints/GI_HeroAdrift.GI_HeroAdrift_C|GetPirateIslandProgress _asgi_hero_adrift) "AskedToHelp"))
    (Variables|Default|SetFunctionEnum "NewEnumerator1")))

(event EventOnInteract
  (params (Interactor :type First%20Person%20Character%20Object%20Reference))
  (switch Utilities|FlowControl|Switch|SwitchonEnumMAFH_Actor2_Function (Variables|Default|GetFunctionEnum)
    (:NewEnumerator0
      (bind _asbp_mango (Utilities|Casting|CastToBP_Mango (Variables|Default|GetMangoRef)))
      (Variables|/Game/Ash/Blueprints/LevelSpecific/PirateIsland/BP_Mango.BP_Mango_C|SetGiveItem _asbp_mango true)
      (Variables|Default|SetFunctionEnum "NewEnumerator1")
      (bind _asfirst_person_character (Utilities|Casting|CastToFirstPersonCharacter (Game|GetPlayerCharacter 0)))
      (Variables|/Game/Ash/Blueprints/Components/HealthComponent.HealthComponent_C|SetCurrentHealth (Variables|/Game/FirstPersonBP/Blueprints/FirstPersonCharacter.FirstPersonCharacter_C|GetHealthComponent _asfirst_person_character) (Variables|/Game/Ash/Blueprints/Components/HealthComponent.HealthComponent_C|GetMaxHealth (Variables|/Game/FirstPersonBP/Blueprints/FirstPersonCharacter.FirstPersonCharacter_C|GetHealthComponent _asfirst_person_character))))
    (:NewEnumerator1
      (bind _asbp_mango_2 (Utilities|Casting|CastToBP_Mango (Variables|Default|GetMangoRef)))
      (Variables|/Game/Billy/DialogueSystemMKII/BPComp_Dialogue.BPComp_Dialogue_C|SetDialogueTree (Variables|/Game/Billy/DialogueSystemMKII/BP_SkeletalMeshDialogue.BP_SkeletalMeshDialogue_C|GetBPComp_Dialogue _asbp_mango_2) "/Game/Ash/Blueprints/LevelSpecific/PirateIsland/BT_BedroomDirections.BT_BedroomDirections")
      (bind _asgi_hero_adrift (Utilities|Casting|CastToGI_HeroAdrift (Game|GetGameInstance)))
      (Default|SaveLevelProgress _asgi_hero_adrift (Variables|/Game/Ash/Blueprints/GI_HeroAdrift.GI_HeroAdrift_C|GetPirateIslandProgress _asgi_hero_adrift) "AskedToHelp")
      (bind _asbp_mango_bed (Utilities|Casting|CastToBP_MangoBed (Variables|Default|GetMangoBedRef)))
      (Collision|SetCollisionResponsetoChannel (Variables|/Game/Ash/Blueprints/LevelSpecific/PirateIsland/BP_MangoBed.BP_MangoBed_C|GetBed_Single _asbp_mango_bed) "ECC_GameTraceChannel3" "ECR_Block"))))

(fn ConstructionScript)