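; Enemy weapon actor that damages the player character when it overlaps them.
; Overlap passes a CanDamage check and a DoOnce gate, then calls DealDamage on its DamageComponent and clears CanDamage.
; ResetDealDamage reopens the DoOnce gate but leaves CanDamage unchanged.
; The construction script picks a random mesh from the integer-keyed WeaponMeshes map for visual variety.
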(event Custom|ResetDealDamage
  (Utilities|FlowControl|DoOnce false) ; enters at Reset
)

(event Collision|EventActorBeginOverlap
  (params (OtherActor :type Actor%20Object%20Reference))
  (if (and (== OtherActor (Game|GetPlayerCharacter 0)) (Variables|Default|GetCanDamage))
    (Utilities|FlowControl|DoOnce false
      (:Completed
        (Default|DealDamage (Variables|Default|GetDamageComponent) OtherActor)
        (Variables|Default|SetCanDamage false)))))

(fn ConstructionScript
  (bind _weaponmeshes (Variables|Default|GetWeaponMeshes))
  (Components|StaticMesh|SetStaticMesh (Variables|Default|GetStaticMesh) (.Value (Utilities|Map|Find _weaponmeshes (Math|Random|RandomIntegerinRange 1 (Utilities|Map|Length _weaponmeshes))))))