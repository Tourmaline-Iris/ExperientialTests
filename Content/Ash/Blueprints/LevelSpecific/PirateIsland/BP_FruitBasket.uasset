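; BP_FruitBasket is an interactable Pirate Island basket where the player deposits fruit they have picked up.
; Picking up fruit makes the basket block a custom collision channel; interacting checks a local flag or GI_HeroAdrift's saved island progress.
; A valid deposit reveals the banana bundle, fires PlayerPutFruitInBasket and stops blocking that channel.
; A separate MangoFruitInBasket event reveals the apple mesh.
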(event Custom|MangoFruitInBasket
  (Development|SetHiddeninGame (Variables|Default|GetSM_MERGED_Apple) false false))

(event Custom|PlayerFruitInBasket
  (Development|SetHiddeninGame (Variables|Default|GetSM_MERGED_banana_bundle) false false)
  (Default|CallPlayerPutFruitinBasket)
  (Variables|Default|SetPlayerFruitPresent true))

(event Custom|PlayerPicksUpFruit
  (Variables|Default|SetPlayerHasFruit true)
  (Collision|SetCollisionResponsetoChannel (Variables|Default|GetSM_MERGED_Basket) "ECC_GameTraceChannel3" "ECR_Block"))

(event EventOnInteract
  (params (Interactor :type First%20Person%20Character%20Object%20Reference))
  (bind _asgi_hero_adrift (Utilities|Casting|CastToGI_HeroAdrift (Game|GetGameInstance)))
  (if (or (Variables|Default|GetPlayerHasFruit) (.Value (Utilities|Map|Find (Variables|/Game/Ash/Blueprints/GI_HeroAdrift.GI_HeroAdrift_C|GetPirateIslandProgress _asgi_hero_adrift) "PlayerHasFruit")))
    (CallFunction|PlayerFruitinBasket)
    (Collision|SetCollisionResponsetoChannel (Variables|Default|GetSM_MERGED_Basket) "ECC_GameTraceChannel3" "ECR_Ignore")))

(fn ConstructionScript)