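; Anchor weapon whose secondary use fires a chained anchor projectile from the first-person player.
; A camera line trace sets the aim of the spawned BP_AnchorProjectile, while the weapon mesh hides and a runtime cable component attaches to the projectile as the chain.
; HookReturned destroys the chain and shows the mesh again.
; PullOther uses a timeline to lerp a given actor toward the player's GripPointSecondary socket.
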(event Custom|HookReturned
  (bind _chain (Variables|Default|GetChain))
  (Utilities|IsValid _chain
    (:Is%20Valid
      (Components|DestroyComponent _chain))
    (:Is%20Not%20Valid
      _))
  (Rendering|SetVisibility (Variables|Default|GetStaticMesh) true false))

(event Custom|PullOther
  (params (Other :type Scene%20Component%20Object%20Reference) (PlayerSkeletalMesh :type Scene%20Component%20Object%20Reference))
  (bind _pulltrack (Timeline|Pull PlayFromStart)
    (:Update
      (Transformation|SetWorldLocation Other (Math|Vector|Lerp(Vector) (Transformation|GetWorldLocation Other) (Transformation|GetSocketLocation PlayerSkeletalMesh "GripPointSecondary") _pulltrack) false false))))

(event EventUseSecondary
  (params (Instigator :type Pawn%20Object%20Reference))
  (bind _staticmesh (Variables|Default|GetStaticMesh))
  (bind _staticmesh_2 (Variables|Default|GetStaticMesh))
  (bind _returnvalue (Transformation|GetWorldTransform _staticmesh_2))
  (bind _returnvalue_2 (Transformation|GetWorldLocation _staticmesh))
  (|CallParentFunction Instigator)
  (bind _asfirst_person_character (Utilities|Casting|CastToFirstPersonCharacter Instigator))
  (bind (_outhit _returnvalue_3) (Collision|LineTraceByChannel (Transformation|GetWorldLocation (Variables|/Game/FirstPersonBP/Blueprints/FirstPersonCharacter.FirstPersonCharacter_C|GetFirstPersonCamera _asfirst_person_character)) (* (Math|Vector|GetForwardVector (Variables|/Game/FirstPersonBP/Blueprints/FirstPersonCharacter.FirstPersonCharacter_C|GetFirstPersonCamera _asfirst_person_character)) 5e+03) "TraceTypeQuery1" false 0 "None" true "(R=1.000000,G=0.000000,B=0.000000,A=1.000000)" "(R=0.000000,G=1.000000,B=0.000000,A=1.000000)" (Utilities|Time|GetWorldDeltaSeconds)))
  (bind _returnvalue_4 (Game|SpawnActorfromClass "/Game/Ash/Blueprints/BP_AnchorProjectile.BP_AnchorProjectile_C" (Math|Transform|MakeTransform _returnvalue_2 (Math|Rotator|FindLookatRotation _returnvalue_2 (Math|Vector|SelectVector (.ImpactPoint (Collision|BreakHitResult _outhit)) (.TraceEnd (Collision|BreakHitResult _outhit)) _returnvalue_3))) "Undefined" self (Variables|/Game/FirstPersonBP/Blueprints/FirstPersonCharacter.FirstPersonCharacter_C|GetSkeletalMesh _asfirst_person_character) _asfirst_person_character))
  (Rendering|SetVisibility _staticmesh_2 false false)
  (bind _returnvalue_5 (AddComponent|AddCableComponent true (Math|Transform|MakeTransform (.location _returnvalue) (.rotation _returnvalue) "1,1,1")))
  (bind _output_get (Variables|Default|SetChain _returnvalue_5))
  (Class|CableComponent|SetAttachEndto _output_get _returnvalue_4 "None" "None"))

(fn ConstructionScript)