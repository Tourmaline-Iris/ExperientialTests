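; BP_FishGoblin is a melee enemy that chases and attacks the player, with randomised body colours set in the construction script.
; PawnSensing drives it: sight starts AIMoveTo or sets attack flags within melee range, while noise turns it toward the sound through a timeline.
; Tick prints health and checks for death, which disables movement and collision, then destroys the actor with a one-in-three chance of a health pickup.
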(event OnSeePawn(PawnSensing)
  (params (Pawn :type Pawn%20Object%20Reference))
  ;[1 1 1] Sees player
  (Variables|Default|SetSeesPlayer (and (== Pawn (Game|GetPlayerCharacter 0)) (not (Variables|Default|GetDead))))
  (Utilities|FlowControl|Sequence
    (:then_0
      (if (> (Transformation|GetDistanceTo (Game|GetPlayerCharacter 0)) (Variables|Default|GetMeleeRange))
        (CallFunction|FollowPlayer)
        (else
          (Variables|Default|SetIsAttacking true)
          (Variables|Default|SetChasingPlayer false))))
    (:then_1
      (Utilities|FlowControl|RetriggerableDelay 0.2)
      (Variables|Default|SetSeesPlayer false))))

(event OnHearNoise(PawnSensing)
  (params (Instigator :type Pawn%20Object%20Reference) (Location :type Vector%20%28by%20ref%29 :default "0, 0, 0") (Volume :type Float%20%28single-precision%29))
  ;[1 1 1] Hear player
  (if (> (Transformation|GetDistanceTo (Game|GetPlayerCharacter 0)) (Variables|Default|GetMeleeRange))
    (Components|Timeline|SetPlayRate (Variables|Default|GetTimeline_LookAtNoise) 1.0)
    (else
      (Components|Timeline|SetPlayRate (Variables|Default|GetTimeline_LookAtNoise) 3.0)))
  (if (Math|Boolean|ANDBoolean (not (Variables|Default|GetDead)) (not (Variables|Default|GetSeesPlayer)) (not (Variables|Default|GetChasingPlayer)))
    (bind _floattrack_lookatnoise (Timeline|Timeline_LookAtNoise PlayFromStart)
      (:Update
        (Transformation|SetActorRotation (Math|Rotator|MakeRotator 0.0 0.0 (Math|Float|Lerp (.yaw (Transformation|GetActorRotation)) (.yaw (Math|Rotator|FindLookatRotation (Transformation|GetActorLocation) Location)) _floattrack_lookatnoise)))))))

(event Custom|FollowPlayer
  ;[1 1 1] Follow player
  (if (Variables|Default|GetSeesPlayer)
    (AI|AIMoveTo self "0, 0, 0" (Game|GetPlayerCharacter 0) (Variables|Default|GetMeleeRange) false
      (:then
        (Variables|Default|SetChasingPlayer true))
      (:OnSuccess
        (Variables|Default|SetIsAttacking true)
        (Variables|Default|SetChasingPlayer false :!label _label))
      (:OnFail
        (goto _label)))))

(event Custom|Die
  (bind _mesh (Variables|Character|GetMesh))
  (bind _returnvalue (Transformation|GetWorldTransform _mesh))
  ;[1 1 1] Enemy Death
  (Variables|Default|SetDead true)
  (Components|Activation|Deactivate (Variables|Character|GetCharacterMovement))
  (bind _asbp_enemy_weapon (Utilities|Casting|CastToBP_EnemyWeapon (Variables|/Script/Engine.ChildActorComponent|GetChildActor (Variables|Default|GetEnemyWeapon))))
  (Collision|SetCollisionEnabled (Variables|Collision|GetCapsuleComponent) "NoCollision")
  ;[1 1 1] Spawn health pickup
  (Utilities|FlowControl|Delay 1.0)
  (if (== (Math|Random|RandomIntegerinRange 1 3) 3)
    (Game|SpawnActorfromClass "/Game/Ash/Blueprints/BP_HealthPickup.BP_HealthPickup_C" (Math|Transform|MakeTransform (Math|Transform|TransformLocation _returnvalue "-80.000000, 0, 0") (Math|Transform|TransformRotation _returnvalue "0, 0, 0")) "Undefined" 0 0))
  (Actor|DestroyActor))

(event EventTick
  (params (DeltaSeconds :type Float%20%28single-precision%29))
  (Development|PrintString (Utilities|String|ToString(Float) (Variables|/Game/Ash/Blueprints/Components/HealthComponent.HealthComponent_C|GetCurrentHealth (Variables|Default|GetHealthComponent))) true true "(R=0.000000,G=0.660000,B=1.000000,A=1.000000)" DeltaSeconds)
  (if (<= (Variables|/Game/Ash/Blueprints/Components/HealthComponent.HealthComponent_C|GetCurrentHealth (Variables|Default|GetHealthComponent)) 0.0)
    (Utilities|FlowControl|DoOnce false
      (:Completed
        (CallFunction|Die)))))

(fn ConstructionScript
  (LocalVariables|SetColourSeed (Math|Random|RandomIntegerinRange 1 (Utilities|Map|Length (Variables|Default|GetMaterialMainColour))))
  (Rendering|Material|SetMaterial (Variables|Character|GetMesh) 0 (.Value (Utilities|Map|Find (Variables|Default|GetMaterialMainColour) (LocalVariables|GetColourSeed))))
  (Rendering|Material|SetMaterial (Variables|Character|GetMesh) 1 (.Value (Utilities|Map|Find (Variables|Default|GetMaterialSecondaryColour) (LocalVariables|GetColourSeed))))
  (Rendering|Material|SetMaterial (Variables|Character|GetMesh) 5 (.Value (Utilities|Map|Find (Variables|Default|GetMaterialGillColour) (LocalVariables|GetColourSeed)))))