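; BP_EnemiesKilledTrigger fires an event once every fish goblin in its assigned EnemiesToTrigger list has been killed.
; On BeginPlay it stores the list length as the required count and binds to each BP_FishGoblin's EnemyKilled dispatcher.
; Each kill increments a counter, and reaching the required count calls the EnemiesInAreaKilled dispatcher.
; A failed cast to BP_FishGoblin stops that binding, yet the entry still counts toward the total.
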(event Custom|CheckEnemysKilled
  (bind _result (Math|Integer|IncrementInt (Variables|Default|GetEnemiesKilled))
    (:%20%20
      (if (== _result (Variables|Default|GetEnemiesRequired))
        (Default|CallEnemiesinAreaKilled)))))

(event EventBeginPlay
  (Variables|Default|SetEnemiesRequired (Utilities|Array|Length (Variables|Default|GetEnemiesToTrigger)))
  (for _array_element (Variables|Default|GetEnemiesToTrigger)
    (bind _asbp_fish_goblin (Utilities|Casting|CastToBP_FishGoblin _array_element))
    (EventDispatchers|BindEventtoEnemyKilled _asbp_fish_goblin (delegate Custom|CheckEnemysKilled))))

(fn ConstructionScript)