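; ParentInteractable is a base Blueprint for objects the first-person player can look at and interact with.
; LookedAt and LookedAtEnd turn the static mesh's custom depth rendering on and off.
; Tick polls the player character's LookAt reference and calls LookedAtEnd on every frame it points elsewhere.
; Interact is an empty event here.
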(event Custom|LookedAt
  (Rendering|SetRenderCustomDepth (Variables|Default|GetStaticMesh) true))

(event Custom|Interact)

(event Custom|LookedAtEnd
  (Rendering|SetRenderCustomDepth (Variables|Default|GetStaticMesh) false))

(event EventTick
  (params (DeltaSeconds :type Float%20%28single-precision%29))
  (bind _asfirst_person_character (Utilities|Casting|CastToFirstPersonCharacter (Game|GetPlayerCharacter 0)))
  (if (not (== (Variables|/Game/FirstPersonBP/Blueprints/FirstPersonCharacter.FirstPersonCharacter_C|GetLookAt _asfirst_person_character) self))
    (CallFunction|LookedatEnd)))

(fn ConstructionScript)