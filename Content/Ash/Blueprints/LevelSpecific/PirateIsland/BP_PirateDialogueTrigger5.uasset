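; Interactable Pirate Island dialogue trigger that either unlocks the anchor or completes the quest.
; On BeginPlay it reads the QuestComplete entry from the game instance's PirateIslandProgress to pick one of two enum-driven interaction functions.
; Function 1 flags Mango to give the item and grants the player the anchor.
; Function 2, picked when the quest is already complete, saves QuestComplete and calls Mirabelle's subconscious quest-complete event.
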(event EventOnInteract
  (params (Interactor :type First%20Person%20Character%20Object%20Reference))
  (switch Utilities|FlowControl|Switch|SwitchonEnumDialogueObjectFunction (Variables|Default|GetEnumFunction)
    (:NewEnumerator0
      (bind _asbp_mango (Utilities|Casting|CastToBP_Mango (Variables|Default|GetMangoRef)))
      (Variables|/Game/Ash/Blueprints/LevelSpecific/PirateIsland/BP_Mango.BP_Mango_C|SetGiveItem _asbp_mango true)
      (bind _asfirst_person_character (Utilities|Casting|CastToFirstPersonCharacter (Game|GetPlayerCharacter 0)))
      (Variables|/Game/FirstPersonBP/Blueprints/FirstPersonCharacter.FirstPersonCharacter_C|SetHasAnchor _asfirst_person_character true)
      (Variables|Default|SetEnumFunction "NewEnumerator0")
      (Development|PrintString "anchor unlocked"))
    (:NewEnumerator1
      (bind _asgi_hero_adrift (Utilities|Casting|CastToGI_HeroAdrift (Game|GetGameInstance)))
      (Default|SaveLevelProgress _asgi_hero_adrift (Variables|/Game/Ash/Blueprints/GI_HeroAdrift.GI_HeroAdrift_C|GetPirateIslandProgress _asgi_hero_adrift) "QuestComplete")
      (Default|CallMirabelle'sSunconsciousQuestComplete)
      (Development|PrintString "quest complete"))))

(event EventBeginPlay
  (bind _asgi_hero_adrift (Utilities|Casting|CastToGI_HeroAdrift (Game|GetGameInstance)))
  (if (.Value (Utilities|Map|Find (Variables|/Game/Ash/Blueprints/GI_HeroAdrift.GI_HeroAdrift_C|GetPirateIslandProgress _asgi_hero_adrift) "QuestComplete"))
    (Variables|Default|SetEnumFunction "NewEnumerator1")
    (else
      (Variables|Default|SetEnumFunction "NewEnumerator0"))))

(fn ConstructionScript)