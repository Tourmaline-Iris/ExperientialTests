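; Anchor hook projectile that launches at HookVelocity, then flies back to the player's secondary grip socket.
; A timeline-driven lerp starts the return once, after a short delay or on hit.
; Hitting a "Hookable" actor also has the owning BP_AnchorWeapon pull it.
; Timeline completion, or the delay-enabled Cone overlapping the player's capsule (behind-player check), resets the secondary weapon, notifies the anchor weapon and destroys the projectile.
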(event OnComponentBeginOverlap(Cone)
  (params (OverlappedComponent :type Primitive%20Component%20Object%20Reference) (OtherActor :type Actor%20Object%20Reference) (OtherComp :type Primitive%20Component%20Object%20Reference) (OtherBodyIndex :type Integer) (bFromSweep :type Boolean) (SweepResult :type Hit%20Result%20Structure%20%28by%20ref%29))
  ;[1 1 1] Check if behind player
  (if (== OtherComp (Variables|/Script/Engine.Character|GetCapsuleComponent (Game|GetPlayerCharacter 0)))
    ;[1 1 1] Reset
    (bind _asfirst_person_character (Utilities|Casting|CastToFirstPersonCharacter (Game|GetPlayerCharacter 0)))
    (Default|ResetSecondaryWeapon _asfirst_person_character (Variables|Default|GetFireRate))
    (bind _asbp_anchor_weapon (Utilities|Casting|CastToBP_AnchorWeapon (Components|GetOwner)))
    (Default|ProjectileReturned _asbp_anchor_weapon)
    (Actor|DestroyActor)))

(event OnComponentHit(SphereCollider)
  (params (HitComponent :type Primitive%20Component%20Object%20Reference) (OtherActor :type Actor%20Object%20Reference) (OtherComp :type Primitive%20Component%20Object%20Reference) (NormalImpulse :type Vector :default "0, 0, 0") (Hit :type Hit%20Result%20Structure%20%28by%20ref%29))
  (Utilities|FlowControl|Sequence
    (:then_0
      ;[1 1 1] Return to player
      (Utilities|FlowControl|DoOnce false
        (:Completed
          (bind _returntrack (Timeline|Return Play)
            (:Update
              (Variables|/Script/Engine.MovementComponent|SetVelocity (Variables|Default|GetProjectileMovement) "0, 0, 0")
              (Transformation|SetActorLocation (Math|Vector|Lerp(Vector) (Transformation|GetWorldLocation (Variables|Default|GetStaticMesh)) (Transformation|GetSocketLocation (Variables|Default|GetPlayerSkeletalMesh) "GripPointSecondary") _returntrack) false false))
            (:Finished
              ;[1 1 1] Reset
              (bind _asfirst_person_character (Utilities|Casting|CastToFirstPersonCharacter (Game|GetPlayerCharacter 0)))
              (Default|ResetSecondaryWeapon _asfirst_person_character (Variables|Default|GetFireRate))
              (bind _asbp_anchor_weapon (Utilities|Casting|CastToBP_AnchorWeapon (Components|GetOwner)))
              (Default|ProjectileReturned _asbp_anchor_weapon)
              (Actor|DestroyActor))))))
    (:then_1
      ;[1 1 1] Pull object
      (if (Actor|ActorHasTag OtherActor "Hookable")
        (bind _asbp_anchor_weapon_2 (Utilities|Casting|CastToBP_AnchorWeapon (Components|GetOwner)))
        (Default|PullOther _asbp_anchor_weapon_2 (Variables|/Script/Engine.Actor|GetRootComponent OtherActor) (Variables|Default|GetPlayerSkeletalMesh))))))

(event EventBeginPlay
  ;[1 1 1] Initialise
  (bind _asfirst_person_character (Utilities|Casting|CastToFirstPersonCharacter (Game|GetInstigator)))
  (Class|PrimitiveComponent|IgnoreComponentwhenMoving (Variables|Default|GetSphereCollider) (Variables|/Script/Engine.Character|GetCapsuleComponent _asfirst_person_character) true)
  ;[1 1 1] Begin return
  (Utilities|FlowControl|Delay 0.2)
  (Collision|SetCollisionEnabled (Variables|Default|GetCone) "QueryOnly")
  ;[1 1 1] Return to player
  (Utilities|FlowControl|DoOnce false
    (:Completed
      (bind _returntrack (Timeline|Return Play)
        (:Update
          (Variables|/Script/Engine.MovementComponent|SetVelocity (Variables|Default|GetProjectileMovement) "0, 0, 0")
          (Transformation|SetActorLocation (Math|Vector|Lerp(Vector) (Transformation|GetWorldLocation (Variables|Default|GetStaticMesh)) (Transformation|GetSocketLocation (Variables|Default|GetPlayerSkeletalMesh) "GripPointSecondary") _returntrack) false false))
        (:Finished
          ;[1 1 1] Reset
          (bind _asfirst_person_character_2 (Utilities|Casting|CastToFirstPersonCharacter (Game|GetPlayerCharacter 0)))
          (Default|ResetSecondaryWeapon _asfirst_person_character_2 (Variables|Default|GetFireRate))
          (bind _asbp_anchor_weapon (Utilities|Casting|CastToBP_AnchorWeapon (Components|GetOwner)))
          (Default|ProjectileReturned _asbp_anchor_weapon)
          (Actor|DestroyActor))))))

(fn ConstructionScript
  (bind _projectilemovement (Variables|Default|GetProjectileMovement))
  (bind _hookvelocity (Variables|Default|GetHookVelocity))
  (Variables|/Script/Engine.ProjectileMovementComponent|SetMaxSpeed _projectilemovement _hookvelocity)
  (Variables|/Script/Engine.ProjectileMovementComponent|SetInitialSpeed _projectilemovement _hookvelocity)
  (Variables|/Script/Engine.MovementComponent|SetVelocity _projectilemovement (Math|Vector|MakeVector _hookvelocity 0.0 0.0))
  (Collision|SetCollisionEnabled (Variables|Default|GetCone) "NoCollision"))