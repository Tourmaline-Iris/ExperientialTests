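; DamageComponent is an actor component that applies its Damage value to a target actor's health.
; DealDamage looks up the target's HealthComponent and subtracts Damage from CurrentHealth, clamped between zero and MaxHealth.
; If that health is flagged as player health and reaches zero, it calls GameOver on the FirstPersonCharacter directly.
; Non-player targets get no death handling here, and BeginPlay and Tick are unused.
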(event EventBeginPlay)

(event EventTick
  (params (DeltaSeconds :type Float%20%28single-precision%29)))

(fn DealDamage
  (params (Target :type Actor%20Object%20Reference))
  (bind _returnvalue (Actor|GetComponentbyClass Target "/Game/Ash/Blueprints/Components/HealthComponent.HealthComponent_C"))
  (Utilities|IsValid _returnvalue
    (:Is%20Valid
      (bind _output_get (Variables|/Game/Ash/Blueprints/Components/HealthComponent.HealthComponent_C|SetCurrentHealth _returnvalue (Math|Float|Clamp(Float) (- (Variables|/Game/Ash/Blueprints/Components/HealthComponent.HealthComponent_C|GetCurrentHealth _returnvalue) (Variables|Default|GetDamage)) 0.0 (Variables|/Game/Ash/Blueprints/Components/HealthComponent.HealthComponent_C|GetMaxHealth _returnvalue))))
      (if (and (Variables|/Game/Ash/Blueprints/Components/HealthComponent.HealthComponent_C|GetIsPlayerHealth _returnvalue) (<= _output_get 0.0))
        (bind _asfirst_person_character (Utilities|Casting|CastToFirstPersonCharacter (Game|GetPlayerCharacter 0)))
        (Default|GameOver _asfirst_person_character))
      (return))))