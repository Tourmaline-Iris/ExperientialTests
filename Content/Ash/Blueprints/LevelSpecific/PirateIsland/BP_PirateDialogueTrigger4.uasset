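; Pirate Island dialogue trigger that, on interact, sends Mirabelle running to her next room.
; BeginPlay reads PirateIslandProgress from GI_HeroAdrift and sets FunctionEnum to Function1 if Mirabelle was helped but the quest is incomplete.
; OnInteract switches on that enum: the first step calls RunToMangoRoom and advances to Function2, which calls RunToBedroom on each later interaction.
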(event EventBeginPlay
  (bind _asgi_hero_adrift (Utilities|Casting|CastToGI_HeroAdrift (Game|GetGameInstance)))
  (if (and (.Value (Utilities|Map|Find (Variables|/Game/Ash/Blueprints/GI_HeroAdrift.GI_HeroAdrift_C|GetPirateIslandProgress _asgi_hero_adrift) "HelpedMirabelle")) (not (.Value (Utilities|Map|Find (Variables|/Game/Ash/Blueprints/GI_HeroAdrift.GI_HeroAdrift_C|GetPirateIslandProgress _asgi_hero_adrift) "QuestComplete"))))
    (Variables|Default|SetFunctionEnum "NewEnumerator0")))

(event EventOnInteract
  (params (Interactor :type First%20Person%20Character%20Object%20Reference))
  (switch Utilities|FlowControl|Switch|SwitchonEnumDialogueObjectFunction (Variables|Default|GetFunctionEnum)
    (:NewEnumerator0
      (bind _asbp_mirabelle (Utilities|Casting|CastToBP_Mirabelle (Variables|Default|GetMirabelleRef)))
      (Default|RuntoMangoRoom _asbp_mirabelle)
      (Variables|Default|SetFunctionEnum "NewEnumerator1"))
    (:NewEnumerator1
      (bind _asbp_mirabelle_2 (Utilities|Casting|CastToBP_Mirabelle (Variables|Default|GetMirabelleRef)))
      (Default|RuntoBedroom _asbp_mirabelle_2))))

(fn ConstructionScript)